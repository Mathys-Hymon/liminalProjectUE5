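; Interactable radio whose handset the player pulls off with a hand movement, triggering a one-time dialogue message.
; Once movement passes a threshold, a gate lets Hold move the handset to the hand, rotating it and scaling it by camera distance.
; A retriggerable delay detects when holding stops, then closes the radio and a timeline eases the handset back into place.
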(event Custom|closeRadio
  (bind _radiohandle (Variables|Default|GetradioHandle))
  (bind _radiohandle_2 (Variables|Default|GetradioHandle))
  (bind _returnvalue (Transformation|GetWorldScale _radiohandle_2))
  (Variables|Default|SetradioOffBlock false)
  (Variables|Default|SetcanGrabRadio false)
  (Utilities|FlowControl|Sequence
    (:then_0
      (Utilities|FlowControl|DoOnce false) ; enters at Reset
    )
    (:then_1
      (Utilities|FlowControl|Gate true) ; enters at Close
    )))

(event EventBeginPlay
  (bind _returnvalue (Rendering|Material|CreateDynamicMaterialInstance (Rendering|Material|GetMaterial (Variables|Default|GetCube) 0) "None" "None" :!class /Script/Engine.KismetMaterialLibrary))
  (Rendering|Material|SetMaterial (Variables|Default|GetCube) 0 _returnvalue))

(event EventHold
  (params (movement :type Vector%202D%20Structure) (handLocation :type Vector :default "0, 0, 0"))
  (bind _radiohandle (Variables|Default|GetradioHandle))
  (bind _radiohandle_2 (Variables|Default|GetradioHandle))
  (bind _returnvalue (Transformation|GetWorldScale _radiohandle_2))
  (Utilities|FlowControl|Sequence
    (:then_0
      (Utilities|FlowControl|DoOnce false
        (:Completed
          (Utilities|FlowControl|Delay 0.3)
          (Variables|Default|SetcanGrabRadio true)
          (Variables|Default|SetinitialScale _returnvalue)
          (Variables|Default|SetnearScale (/ _returnvalue 4.0)))))
    (:then_1
      (Utilities|FlowControl|Gate true :!label _label
        (:Exit
          (Transformation|SetWorldLocation (Variables|Default|GetradioHandle) handLocation false false)
          (Utilities|FlowControl|Sequence
            (:then_0
              (Utilities|FlowControl|DoOnce false
                (:Completed
                  (Class|BPIPlayerController|PlayDialogue(Message) (Game|GetPlayerController 0) (Variables|Default|Getdialogues)))))
            (:then_1
              (Transformation|SetRelativeRotation (Variables|Default|GetradioHandle) (Math|Interpolation|RInterpTo (Variables|/Script/Engine.SceneComponent|GetRelativeRotation (Variables|Default|GetradioHandle)) (Math|Rotator|FindLookatRotation (* (Math|Vector|GetForwardVector (Camera|GetCameraRotation (Game|GetPlayerCameraManager 0))) -1.0) (Math|Vector|MakeVector 0.0 0.0 0.0)) (Utilities|Time|GetWorldDeltaSeconds) 6.0) false false)
              (Transformation|SetWorldScale3D (Variables|Default|GetradioHandle) (Math|Vector|Lerp(Vector) (Variables|Default|GetnearScale) (Variables|Default|GetinitialScale) (Math|Float|Clamp(Float) (/ (- (/ (Math|Vector|Distance(Vector) (Transformation|GetWorldLocation (Variables|Default|GetradioHandle)) (Camera|GetCameraLocation (Game|GetPlayerCameraManager 0))) 24.0) 1.0) 1e+01))))
              (Variables|Default|SetradioOffBlock true)
              (Utilities|FlowControl|RetriggerableDelay 0.1)
              (CallFunction|CloseRadio)
              (bind _alpha (Timeline|goBackInPlace PlayFromStart)
                (:Update
                  (Transformation|SetRelativeLocation _radiohandle (Math|Vector|Lerp(Vector) (Variables|/Script/Engine.SceneComponent|GetRelativeLocation _radiohandle) "0, 0, 0" _alpha) false true)
                  (Transformation|SetWorldScale3D _radiohandle (Math|Vector|Lerp(Vector) (Transformation|GetWorldScale _radiohandle) (Variables|Default|GetinitialScale) _alpha))
                  (Transformation|SetRelativeRotation _radiohandle (Math|Rotator|Lerp(Rotator) (Variables|/Script/Engine.SceneComponent|GetRelativeRotation _radiohandle) "0, 0, 0" _alpha true) false false))))))))
    (:then_2
      (if (and (> (Math|Vector2D|Vector2DLength movement) 1e+01) (Variables|Default|GetcanGrabRadio))
        (goto _label Open)))))

(fn ConstructionScript
  (|CallParentFunction))

(fn HandleLocation
  (return (Math|Vector|SelectVector "0, 0, 0" (Transformation|GetWorldLocation (Variables|Default|GetradioHandle)) (Variables|Default|GetradioOffBlock))))