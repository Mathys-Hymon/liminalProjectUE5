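; BP_TV is an interactable TV whose handle the player twists to advance a channel counter.
; Hold turns horizontal movement into a hand rotation offset and, past a threshold, increments TvChannel through a DoOnce that resets after a delay.
; HandleLocation places the hand in front of the handle mesh, pitched by channel count and offset, while InteractBounds exposes that mesh's bounds, shifted forward.
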(event EventBeginPlay
  (|CallParentFunction) ; This node is disabled and will not be called.\nDrag off pins to build functionality.
)

(event Collision|EventActorBeginOverlap
  (params (OtherActor :type Actor%20Object%20Reference)))

(event EventTick
  (params (DeltaSeconds :type Float%20%28single-precision%29))
  (|CallParentFunction DeltaSeconds))

(event EventHold
  (params (movement :type Vector%202D%20Structure) (handLocation :type Vector :default "0, 0, 0"))
  (Variables|Default|SethandRotationOffset (* (.x movement) 0.1))
  (if (> (.x movement) 65.0)
    (Utilities|FlowControl|DoOnce false :!label _label
      (:Completed
        (Math|Integer|IncrementInt (Variables|Default|GettvChannel)
          (:%20%20
            (Utilities|FlowControl|Delay 3.0)
            (goto _label Reset)))))))

(fn ConstructionScript
  (|CallParentFunction))

(fn HandleLocation
  (return (+ (Transformation|GetWorldLocation (Variables|Default|GetSM_TVHandle)) (* (Transformation|GetActorForwardVector) 4e+01)) (Math|Rotator|MakeRotator 0.0 (+ (* -25.0 (Variables|Default|GettvChannel)) (* (Variables|Default|GethandRotationOffset) -1.0)) 0.0)))

(fn InteractBounds
  (bind _sm_tvhandle (Variables|Default|GetSM_TVHandle))
  (bind (_origin _boxextent) (Collision|GetComponentBounds _sm_tvhandle))
  (return (+ _origin (* (Transformation|GetActorForwardVector) 2e+01)) _boxextent))