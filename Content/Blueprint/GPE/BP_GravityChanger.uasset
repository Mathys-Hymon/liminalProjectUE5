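; BP_GravityChanger is a trigger volume that sets a player's gravity to GravityDirection through BPI_Player.
; The first player overlap of PlayerDetection applies it behind a DoOnce that is never reset, saving the previous gravity when ResetGravityWhenExit is set.
; With that flag, every player exit restores the saved gravity.
; The construction script previews the vector with an arrow, scaled by magnitude and hidden when zero.
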(event OnComponentBeginOverlap(playerDetection)
  (params (OverlappedComponent :type Primitive%20Component%20Object%20Reference) (OtherActor :type Actor%20Object%20Reference) (OtherComp :type Primitive%20Component%20Object%20Reference) (OtherBodyIndex :type Integer) (bFromSweep :type Boolean) (SweepResult :type Hit%20Result%20Structure%20%28by%20ref%29))
  (if (Utilities|DoesObjectImplementInterface OtherActor "/Game/Blueprint/BPI/BPI_Player.BPI_Player_C")
    (Utilities|FlowControl|DoOnce false
      (:Completed
        (if (Variables|Default|GetresetGravityWhenExit)
          (bind _gravityfactor (Class|BPIPlayer|GetGravity(Message) OtherActor))
          (Variables|Default|SetpreviousGravity _gravityfactor))
        (Class|BPIPlayer|SetGravity(Message) OtherActor (Variables|Default|GetgravityDirection))))))

(event OnComponentEndOverlap(playerDetection)
  (params (OverlappedComponent :type Primitive%20Component%20Object%20Reference) (OtherActor :type Actor%20Object%20Reference) (OtherComp :type Primitive%20Component%20Object%20Reference) (OtherBodyIndex :type Integer))
  (if (and (Utilities|DoesObjectImplementInterface OtherActor "/Game/Blueprint/BPI/BPI_Player.BPI_Player_C") (Variables|Default|GetresetGravityWhenExit))
    (Class|BPIPlayer|SetGravity(Message) OtherActor (Variables|Default|GetpreviousGravity))))

(event EventBeginPlay)

(event Collision|EventActorBeginOverlap
  (params (OtherActor :type Actor%20Object%20Reference)))

(event EventTick
  (params (DeltaSeconds :type Float%20%28single-precision%29)))

(fn ConstructionScript
  (bind _arrow (Variables|Default|GetArrow))
  (bind _gravitydirection (Variables|Default|GetgravityDirection))
  (bind (_x _y _z) (Math|Vector|BreakVector _gravitydirection))
  (Transformation|SetWorldRotation _arrow (Math|Conversions|RotationFromXVector _gravitydirection) false false)
  (Rendering|SetVisibility _arrow (Math|Boolean|ORBoolean (!= _x 0.0) (!= _y 0.0) (!= _z 0.0)) false)
  (Variables|/Script/Engine.ArrowComponent|SetArrowSize _arrow (Math|Vector|VectorLength (Variables|Default|GetgravityDirection))))