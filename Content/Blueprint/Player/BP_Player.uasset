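; First-person player with lagged look and movement and a sprite hand for grabbing and interacting with objects.
; Look input accumulates into a decaying vector that turns the camera, or moves the hand within limits when hand mode is on.
; Clicking sphere-traces through the hand and sends hold messages to non-collectibles, which can return a location to pull the hand toward.
; Traces also pick the hand sprite; timelines animate walk sway and hand returns.
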(event EventBeginPlay
  ;[0 0.5947 1] Begin Play
  (Components|Timeline|SetPlayRate (Variables|Default|GetHandMovement) 0.4)
  (bind _returnvalue (UserInterface|CreateWidget "/Game/Blueprint/UI/WBP_Player.WBP_Player_C"))
  (bind _output_get (Variables|Default|SetwidgetRef _returnvalue))
  (UserInterface|SetWidget (Variables|Default|GetWidget) _output_get))

(event EventTick
  (params (DeltaSeconds :type Float%20%28single-precision%29))
  ;[1 0 0] Tick
  (|cameraLagMovement)
  (|MovementLag)
  (|setHandSprite))

(event EventEndClick
  (Variables|Hand|SetgrabbedObject 0)
  (if (> (Math|Vector|VectorLength (Variables|Hand|GetlastHandLocation)) 0.1)
    (bind _alpha (Timeline|releaseHandTimeline PlayFromStart)
      (:Update
        (if (Variables|Hand|GethandEnable)
          (Transformation|SetWorldLocation (Variables|Default|GethandPosition) (Math|Vector|Lerp(Vector) (Transformation|GetWorldLocation (Variables|Default|GethandPosition)) (Variables|Hand|GetlastHandLocation) _alpha) false false))))))

(event EventMove
  (params (axis :type Vector%202D%20Structure))
  (bind _returnvalue (Utilities|Time|GetWorldDeltaSeconds))
  (bind _handposition (Variables|Default|GethandPosition))
  (bind _relativelocation (Variables|/Script/Engine.SceneComponent|GetRelativeLocation _handposition))
  ;[0 0 0] GetMovementInput
  (Variables|Movement|SetmovementVelocity axis)
  (if (not (Variables|Input|GetinputPressed))
    ;[0 0 0] StartMovingHand
    (Variables|Input|SetinputPressed true)
    (Components|Timeline|SetNewTime (Variables|Default|GetHandMovement) 0.25)
    (Audio|Components|Audio|Stop (Variables|Default|GetMoveHandBack))
    (bind (_direction _alphay _alphaz) (Timeline|HandMovement Play)
      (:Update
        (Transformation|SetRelativeLocation _handposition (Math|Vector|MakeVector 13.0 (Math|Interpolation|FInterpTo (.y _relativelocation) _alphay _returnvalue 3.0) (Math|Interpolation|FInterpTo (.z _relativelocation) _alphaz _returnvalue 3.0)) false false)))))

(event EventStopMovement
  (bind _returnvalue (Utilities|Time|GetWorldDeltaSeconds))
  (bind _handposition (Variables|Default|GethandPosition))
  (bind _relativelocation (Variables|/Script/Engine.SceneComponent|GetRelativeLocation _handposition))
  (Variables|Input|SetinputPressed false)
  ;[0 0 0] StartMovingHand
  (Utilities|FlowControl|Sequence
    (:then_0
      (bind (_direction _alphay _alphaz) (Timeline|HandMovement Stop)
        (:Update
          (Transformation|SetRelativeLocation _handposition (Math|Vector|MakeVector 13.0 (Math|Interpolation|FInterpTo (.y _relativelocation) _alphay _returnvalue 3.0) (Math|Interpolation|FInterpTo (.z _relativelocation) _alphaz _returnvalue 3.0)) false false))))
    (:then_1
      ;[0 0 0] Reset Hand Location When Movement Stop
      (Utilities|FlowControl|DelayUntilNextTick)
      (if (not (Variables|Hand|GethandEnable))
        (bind _alpha (Timeline|MoveHandBack PlayFromStart)
          (:Update
            (Variables|Hand|SetlastHandLocation "0, 0, 0")
            (Transformation|SetRelativeLocation (Variables|Default|GethandPosition) (Math|Vector|Lerp(Vector) (Variables|/Script/Engine.SceneComponent|GetRelativeLocation (Variables|Default|GethandPosition)) "13.000000,0.000000,0.054000" _alpha) false false)))))))

(event EventLook
  (params (axis :type Vector%202D%20Structure))
  ;[0 0 0] GetInputCamera
  (Variables|Camera|SetheadMovementLag (+ axis (Variables|Camera|GetheadMovementLag))))

(event EventEnableHand
  (params (enable :type Boolean))
  ;[0 0 0] PlayerCanModeHand
  (bind _output_get (Variables|Hand|SethandEnable enable))
  (if (not _output_get)
    (Components|Timeline|PlayfromStart (Variables|Default|GetMoveHandBack))
    (Variables|Camera|SetheadMovementLag "")))

(event EventIsClicking
  (bind _handsprite (Variables|Default|GetHandSprite))
  (bind _returnvalue (Transformation|GetWorldLocation _handsprite))
  ;[0 0 0] Check ClickObject
  (Utilities|IsValid (Variables|Hand|GetgrabbedObject)
    (:Is%20Valid
      (if (not (Utilities|DoesObjectImplementInterface (.HitActor (Collision|BreakHitResult (stale _outhit))) "/Game/Blueprint/BPI/BPI_Collectible.BPI_Collectible_C")) :!label _label
        (Class|BPIInteractable|Hold(Message) (stale _output_get) (Variables|Camera|GetheadMovementLag) (+ (Transformation|GetWorldLocation (Variables|Default|GetHandSprite)) (Math|Vector|GetForwardVector (Variables|Default|GetCamera))))))
    (:Is%20Not%20Valid
      (bind (_outhit _returnvalue_2) (Collision|SphereTraceByChannel _returnvalue (+ _returnvalue (* (Math|Vector|GetForwardVector (Math|Rotator|FindLookatRotation (Transformation|GetWorldLocation (Variables|Default|GetCamera)) _returnvalue)) 2e+02)) 3.0 "TraceTypeQuery1" false 0 "ForOneFrame"))
      (if _returnvalue_2
        (bind _output_get (Variables|Hand|SetgrabbedObject (.HitActor (Collision|BreakHitResult _outhit))))
        (goto _label)
        (else
          (Variables|Hand|SetgrabbedObject 0))))))

(event EventSetPostProcess
  (params (mat :type Material%20Instance%20Object%20Reference))
  ;[0 0 0] Set Post Process
  (Utilities|IsValid mat
    (:Is%20Valid
      (Variables|/Script/Engine.CameraComponent|SetPostProcessSettings (Variables|Default|GetCamera) (Utilities|Struct|MakePostProcessSettings (Utilities|Struct|MakeWeightedBlendables (Utilities|Array|MakeArray (Utilities|Struct|MakeWeightedBlendable 1.0 mat))))))))

(fn ConstructionScript)

(fn SetHandState
  (params (newState :type Enum_Hand%20Enum :default "NewEnumerator0"))
  (if (not (Utilities|Enum|Equal(Enum) newState (Variables|Hand|GethandState)))
    (Variables|Hand|SethandState newState)))

(event Custom|ResethandLoc
  (Utilities|FlowControl|DoOnce false) ; enters at Reset
)

(fn GetWidgetRef
  (return (Variables|Default|GetwidgetRef)))